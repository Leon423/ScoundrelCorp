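; BP_PlayerController is a player controller that puts the HUD widgets on screen when it possesses a pawn.
; On possession of a locally controlled pawn, it creates WBP_Crosshair and WBP_HealthIndicator and adds both to the viewport.
; It keeps a reference only to the health indicator, which UnPossess removes from its parent; the crosshair is not removed here.
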(event `self.ReceiveBeginPlay`)

(event `self.ReceivePossess`
  (params (PossessedPawn :type "Pawn Object Reference"))
  (if (`Pawn.IsLocallyControlled` PossessedPawn)
    (`|ExecutionSequence`
      (:`then_0`
        (bind _returnvalue (`|CreateWidget` "/Game/UI/WBP_Crosshair.WBP_Crosshair_C"))
        (`UserWidget.AddToViewport` _returnvalue 0))
      (:`then_1`
        (bind _returnvalue_2 (`|CreateWidget` "/Game/UI/WBP_HealthIndicator.WBP_HealthIndicator_C"))
        (bind _output_get (set `self.Health Indicator` _returnvalue_2))
        (`UserWidget.AddToViewport` _output_get 0)))))

(event `self.ReceiveUnPossess`
  (params (UnpossessedPawn :type "Pawn Object Reference"))
  (`Widget.RemoveFromParent` (`self.Health Indicator`)))

(fn `UserConstructionScript`)